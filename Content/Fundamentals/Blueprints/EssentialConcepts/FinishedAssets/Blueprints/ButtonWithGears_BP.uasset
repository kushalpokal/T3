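; ButtonWithGears_BP is a tutorial Blueprint of a button that spins three gears while something overlaps its collision component.
; Begin and end overlap toggle a flag and play or reverse a timeline that moves the button on Z and lerps its emissive color.
; The construction script creates the dynamic material instance for that glow.
; While active, Tick rotates the gears at a frame-rate-independent speed, with two turning opposite to the first.
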(event OnComponentBeginOverlap(CollisionComp)
  (params (OverlappedComponent :type Primitive%20Component%20Object%20Reference) (OtherActor :type Actor%20Object%20Reference) (OtherComp :type Primitive%20Component%20Object%20Reference) (OtherBodyIndex :type Integer) (bFromSweep :type Boolean) (SweepResult :type Hit%20Result%20Structure%20%28by%20ref%29))
  (Variables|Default|SetOn/off true)
  (bind (_direction _press _glow) (Timeline|Timeline_0 Play) ; Timeline for animating the button press
    (:Update
      (Transformation|SetRelativeLocation (Variables|Default|GetButton) (Math|Vector|MakeVector 0.0 0.0 _press) false false) ; Move button up/down
      (Rendering|Material|SetVectorParameterValue (Variables|Default|GetButton%20material) "Emissive" (Math|Color|Lerp(LinearColor) :B "(R=0.600000,G=0.329323,B=0.000000,A=1.000000)" :Alpha _glow) :!class /Script/Engine.MaterialInstanceDynamic) ; Change emissive color of the button
    )))

(event OnComponentEndOverlap(CollisionComp)
  (params (OverlappedComponent :type Primitive%20Component%20Object%20Reference) (OtherActor :type Actor%20Object%20Reference) (OtherComp :type Primitive%20Component%20Object%20Reference) (OtherBodyIndex :type Integer))
  (Variables|Default|SetOn/off false)
  (bind (_direction _press _glow) (Timeline|Timeline_0 Reverse) ; Timeline for animating the button press
    (:Update
      (Transformation|SetRelativeLocation (Variables|Default|GetButton) (Math|Vector|MakeVector 0.0 0.0 _press) false false) ; Move button up/down
      (Rendering|Material|SetVectorParameterValue (Variables|Default|GetButton%20material) "Emissive" (Math|Color|Lerp(LinearColor) :B "(R=0.600000,G=0.329323,B=0.000000,A=1.000000)" :Alpha _glow) :!class /Script/Engine.MaterialInstanceDynamic) ; Change emissive color of the button
    )))

(event EventTick
  (params (DeltaSeconds :type Float%20%28single-precision%29))
  (Variables|Default|SetDelta%20seconds DeltaSeconds) ; Update the time between frames for use later
  (if (Variables|Default|GetOn/off) ; Only proceed if the gears have been activated
    (Transformation|AddLocalRotation (Variables|Default|GetGear%201) (Math|Rotator|MakeRotator 0.0 0.0 (* (Variables|Default|GetRotation%20Speed) (Variables|Default|GetDelta%20seconds))) false false)
    (Transformation|AddLocalRotation (Variables|Default|GetGear%202) (Math|Rotator|MakeRotator 0.0 0.0 (* (* (Variables|Default|GetRotation%20Speed) -1.0) (Variables|Default|GetDelta%20seconds))) false false)))

(fn ConstructionScript
  (bind _returnvalue (Rendering|Material|CreateDynamicMaterialInstance (Variables|Default|GetButton) 0 0 "None" :!class /Script/Engine.PrimitiveComponent)) ; Make and apply a dynamic material instance for the button
  (Variables|Default|SetButton%20material _returnvalue) ; Set the material as a variable for animating
)